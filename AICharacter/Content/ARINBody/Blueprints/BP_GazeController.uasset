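; Gaze controller actor that turns the ARINBody character's head and eyes toward a selectable, lockable target from its object array.
; Each tick it clamps and interpolates look-at rotations into per-controller anim blueprint maps, with eyes generally covering what the head rotation leaves over.
; Gaze and Relax ramp that controller's blend alpha down or up.
; Other functions adjust speed, freeze the angle once reached, or reset all controllers.
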(event `self.ReceiveBeginPlay`
  (bind _outactors (`GameplayStatics.GetAllActorsOfClass` "/Game/ARINBody/Blueprints/CH_ARINBody.CH_ARINBody_C"))
  (for _array_element _outactors
    (set `self.CharacterRef` _array_element)
    (bind _asbp_arinbody_anim_blueprint (cast `/Game/ARINBody/Blueprints/BP_ARINBody_AnimBlueprint` (`SkeletalMeshComponent.GetAnimInstance` (`Character.Mesh` _array_element))))
    (set `self.AnimBPref` _asbp_arinbody_anim_blueprint)
    (set `self.LookatObjectID` (`self.ControllerNum`))))

(event `self.ReceiveTick`
  (params (DeltaSeconds :type "Float (single-precision)"))
  (bind _controllernum (`self.ControllerNum`))
  (bind _animbpref (`self.AnimBPref`))
  (bind _characterref (`self.CharacterRef`))
  (bind _controllernum_2 (`self.ControllerNum`))
  (bind _animbpref_2 (`self.AnimBPref`))
  (bind _controllernum_3 (`self.ControllerNum`))
  (bind _controllernum_4 (`self.ControllerNum`))
  (bind _controllerblendalphaarray (`/Game/ARINBody/Blueprints/BP_ARINBody_AnimBlueprint.ControllerBlendAlphaArray` (`self.AnimBPref`)))
  (bind _controllerblendalphaarray_2 (`/Game/ARINBody/Blueprints/BP_ARINBody_AnimBlueprint.ControllerBlendAlphaArray` (`self.AnimBPref`)))
  (bind _controllerblendalphaarray_3 (`/Game/ARINBody/Blueprints/BP_ARINBody_AnimBlueprint.ControllerBlendAlphaArray` (`self.AnimBPref`)))
  (bind _controllerblendalphaarray_4 (`/Game/ARINBody/Blueprints/BP_ARINBody_AnimBlueprint.ControllerBlendAlphaArray` (`self.AnimBPref`)))
  (bind (_value _returnvalue) (`BlueprintMapLibrary.Map_Find` (`/Game/ARINBody/Blueprints/CH_ARINBody.ObjectArray` _characterref) (`self.LookatObjectID`)))
  (bind _returnvalue_2 (cast `/Game/ARINBody/Data/ControllerNameEnum` (`KismetMathLibrary.Conv_IntToByte` (`self.ControllerNum`))))
  (bind _returnvalue_3 (cast `/Game/ARINBody/Data/ControllerNameEnum` (`KismetMathLibrary.Conv_IntToByte` (`self.ControllerNum`))))
  (`|ExecutionSequence`
    (:`then_0`
      (if _returnvalue
        (set `self.LookTarget` _value)
        (else
          (set `self.LookTarget` (`BlueprintMapLibrary.Map_Find` (`/Game/ARINBody/Blueprints/CH_ARINBody.ObjectArray` _characterref) (`self.ControllerNum`)))))
      (if (not (and (`self.IsFixed`) (`self.IsGazeComplete`)))
        (bind (_outheadlookatrotation _outeyelookatrotation) (`self.CalculateLookRotations` (`Character.Mesh` (`self.CharacterRef`)) "Bip-Head" (`self.LookTarget`) (`BlueprintMapLibrary.Map_Find` (`/Game/ARINBody/Blueprints/BP_ARINBody_AnimBlueprint.HeadRotationConstraint` _animbpref) _returnvalue_3) (`BlueprintMapLibrary.Map_Find` (`/Game/ARINBody/Blueprints/BP_ARINBody_AnimBlueprint.EyeRotationConstraint` _animbpref) _returnvalue_3) (`BlueprintMapLibrary.Map_Find` (`/Game/ARINBody/Blueprints/BP_ARINBody_AnimBlueprint.HeadLookAtRotator` _animbpref) _returnvalue_3) (`BlueprintMapLibrary.Map_Find` (`/Game/ARINBody/Blueprints/BP_ARINBody_AnimBlueprint.EyeLookAtRotator` _animbpref) _returnvalue_3)))
        (`BlueprintMapLibrary.Map_Add` (`/Game/ARINBody/Blueprints/BP_ARINBody_AnimBlueprint.EyeLookAtRotator` _animbpref_2) _returnvalue_2 _outeyelookatrotation)
        (`BlueprintMapLibrary.Map_Add` (`/Game/ARINBody/Blueprints/BP_ARINBody_AnimBlueprint.HeadLookAtRotator` _animbpref_2) _returnvalue_2 _outheadlookatrotation)))
    (:`then_1`
      (if (`self.GazeFlag`)
        (`KismetArrayLibrary.Array_Set` _controllerblendalphaarray_3 _controllernum (- (`|GetArrayItem` _controllerblendalphaarray_3 _controllernum) (`GameplayStatics.GetWorldDeltaSeconds`)))
        (if (<= (`|GetArrayItem` _controllerblendalphaarray_4 _controllernum_2) 0.0)
          (set `self.GazeFlag` false)
          (`KismetArrayLibrary.Array_Set` _controllerblendalphaarray_4 _controllernum_2))))
    (:`then_2`
      (if (`self.RelaxFlag`)
        (`KismetArrayLibrary.Array_Set` _controllerblendalphaarray_2 _controllernum_3 (+ (/ (`GameplayStatics.GetWorldDeltaSeconds`) (`self.RelaxTime`)) (`|GetArrayItem` _controllerblendalphaarray_2 _controllernum_3)))
        (if (>= (`|GetArrayItem` _controllerblendalphaarray _controllernum_4) 1.0)
          (set `self.RelaxFlag` false)
          (`KismetArrayLibrary.Array_Set` _controllerblendalphaarray _controllernum_4 1.0))))))

(fn `CalculateLookRotations`
  (params (CharacterMesh :type "SkeletalMeshComponent Object Reference") (SourceBone :type Name) (LookAtTarget :type "Vector Structure") (HeadRotationConstraint :type "/Game/ARINBody/Data/RotationConstraint Structure") (EyeRotationConstraint :type "/Game/ARINBody/Data/RotationConstraint Structure") (InHeadLookAtRotation :type "Rotator Structure") (InEyeLookAtRotation :type "Rotator Structure"))
  (returns (OutHeadLookAtRotation :type "Rotator Structure") (OutEyeLookAtRotation :type "Rotator Structure"))
  (locals (NewLocalVar_0 :type "Rotator Structure" :default (struct)))
  (bind (_minroll _maxroll _minpitch _maxpitch _minyaw _maxyaw _speed) (break `/Game/ARINBody/Data/RotationConstraint` HeadRotationConstraint))
  (bind (_minroll_2 _maxroll_2 _minpitch_2 _maxpitch_2 _minyaw_2 _maxyaw_2 _speed_2) (break `/Game/ARINBody/Data/RotationConstraint` EyeRotationConstraint))
  (bind _outrotator (`self.RemapLookAtRotator` (`KismetMathLibrary.MakeRotator` (- (.roll (`KismetMathLibrary.FindLookAtRotation` (`SceneComponent.GetSocketLocation` CharacterMesh SourceBone) LookAtTarget)) (.roll (struct))) (* (- (.pitch (`KismetMathLibrary.FindLookAtRotation` (`SceneComponent.GetSocketLocation` CharacterMesh SourceBone) LookAtTarget)) (.pitch (struct))) -1.0) (- (.yaw (`KismetMathLibrary.FindLookAtRotation` (`SceneComponent.GetSocketLocation` CharacterMesh SourceBone) LookAtTarget)) (.yaw (struct))))))
  (bind _output_get (set `self.RawLookatRotation` _outrotator))
  (bind _returnvalue (`KismetMathLibrary.MakeRotator` (.roll _output_get) (`KismetMathLibrary.FClamp` (.pitch _output_get) _minpitch _maxpitch) (`KismetMathLibrary.FClamp` (.yaw _output_get) _minyaw _maxyaw)))
  (bind _returnvalue_2 (== _returnvalue InHeadLookAtRotation :`ErrorTolerance` 1.0))
  (if (not _returnvalue_2)
    (set `self.IsGazeChange` true)
    (set `self.IsGazeComplete` false))
  (if (and _returnvalue_2 (`self.IsGazeChange`))
    (set `self.IsGazeComplete` true)
    (set `self.IsGazeChange` false)
    (if (`self.ToBeFixed`)
      (set `self.IsFixed` true)
      (set `self.ToBeFixed` false)))
  (bind _output_get_2 (set `self.NewHeadLookAtRotation` (`KismetMathLibrary.RInterpTo` InHeadLookAtRotation _returnvalue (`GameplayStatics.GetWorldDeltaSeconds`) _speed)))
  (if (== (`self.ControllerNum`) (`KismetMathLibrary.Conv_ByteToInt` (enumliteral `/Game/ARINBody/Data/ControllerNameEnum` "NewEnumerator20")))
    (set `self.TempEyeRotate` (`self.RawLookatRotation`))
    (else
      (set `self.TempEyeRotate` (`KismetMathLibrary.MakeRotator` (.roll (`self.RawLookatRotation`)) (- (.pitch (`self.RawLookatRotation`)) (.pitch _output_get_2)) (- (.yaw (`self.RawLookatRotation`)) (.yaw _output_get_2))))))
  (set `self.NewEyeLookAtRotation` (`KismetMathLibrary.RInterpTo` InEyeLookAtRotation (`KismetMathLibrary.MakeRotator` (.roll (`self.TempEyeRotate`)) (`KismetMathLibrary.FClamp` (.pitch (`self.TempEyeRotate`)) _minpitch_2 _maxpitch_2) (`KismetMathLibrary.FClamp` (.yaw (`self.TempEyeRotate`)) _minyaw_2 _maxyaw_2)) (`GameplayStatics.GetWorldDeltaSeconds`) _speed_2))
  (return (`self.NewHeadLookAtRotation`) (`self.NewEyeLookAtRotation`)))

(fn `DualGaze`
  (params (ObjectID :type Integer))
  (bind _animbpref (`self.AnimBPref`))
  (bind _animbpref_2 (`self.AnimBPref`))
  (bind _eyelookatrotator (`/Game/ARINBody/Blueprints/BP_ARINBody_AnimBlueprint.EyeLookAtRotator` _animbpref_2))
  (bind (_returnvalue_location _returnvalue_rotation) (`KismetMathLibrary.BreakTransform` (`SceneComponent.GetSocketTransform` (`Character.Mesh` (`self.CharacterRef`)) "Bip-Head" "RTS_ParentBoneSpace")))
  (bind _returnvalue (cast `/Game/ARINBody/Data/ControllerNameEnum` (`KismetMathLibrary.Conv_IntToByte` (`self.ControllerNum`))))
  (bind _output_get (set `self.NewVar_2` (`KismetMathLibrary.MakeRotator` (.pitch _returnvalue_rotation) (.yaw _returnvalue_rotation) (.roll _returnvalue_rotation))))
  (`BlueprintMapLibrary.Map_Add` (`/Game/ARINBody/Blueprints/BP_ARINBody_AnimBlueprint.HeadLookAtRotator` _animbpref_2) _returnvalue (* _output_get -1))
  (`BlueprintMapLibrary.Map_Add` _eyelookatrotator _returnvalue (`BlueprintMapLibrary.Map_Find` _eyelookatrotator "NewEnumerator13"))
  (`KismetArrayLibrary.Array_Set` (`/Game/ARINBody/Blueprints/BP_ARINBody_AnimBlueprint.ControllerBlendAlphaArray` (`self.AnimBPref`)) (`self.ControllerNum`))
  (`/Game/ARINBody/Blueprints/BP_DataController.DoInterruptRelax` (`/Game/ARINBody/Blueprints/BP_ARINBody_AnimBlueprint.Head1ControllerRef` _animbpref))
  (`/Game/ARINBody/Blueprints/BP_DataController.DoInterruptRelax` (`/Game/ARINBody/Blueprints/BP_ARINBody_AnimBlueprint.Head2ControllerRef` _animbpref))
  (`self.SetTarget` ObjectID))

(fn `FixGazeAngle`
  (if (`self.IsGazeComplete`)
    (set `self.IsFixed` true)
    (else
      (set `self.ToBeFixed` true))))

(fn `Gaze`
  (set `self.GazeFlag` true)
  (set `self.RelaxFlag` false))

(fn `GazeSpeed`
  (params (Speed :type String))
  (bind _animbpref (`self.AnimBPref`))
  (bind _eyerotationconstraint (`/Game/ARINBody/Blueprints/BP_ARINBody_AnimBlueprint.EyeRotationConstraint` _animbpref))
  (bind _headrotationconstraint (`/Game/ARINBody/Blueprints/BP_ARINBody_AnimBlueprint.HeadRotationConstraint` _animbpref))
  (bind _returnvalue (cast `/Game/ARINBody/Data/ControllerNameEnum` (`KismetMathLibrary.Conv_IntToByte` (`self.ControllerNum`))))
  (switch `string` Speed
    (:`0.5`
      (`BlueprintMapLibrary.Map_Add` _headrotationconstraint _returnvalue (make `/Game/ARINBody/Data/RotationConstraint` 0.0 0.0 -40.0 40.0 -40.0 40.0 2.0))
      (`BlueprintMapLibrary.Map_Add` _eyerotationconstraint _returnvalue (make `/Game/ARINBody/Data/RotationConstraint` 0.0 0.0 -30.0 30.0 -30.0 30.0 1.0)))
    (:`1.0`
      (`BlueprintMapLibrary.Map_Add` _headrotationconstraint _returnvalue (make `/Game/ARINBody/Data/RotationConstraint` 0.0 0.0 -40.0 40.0 -40.0 40.0 4.0))
      (`BlueprintMapLibrary.Map_Add` _eyerotationconstraint _returnvalue (make `/Game/ARINBody/Data/RotationConstraint` 0.0 0.0 -30.0 30.0 -30.0 30.0 2.0)))
    (:`1.5`
      (`BlueprintMapLibrary.Map_Add` _headrotationconstraint _returnvalue (make `/Game/ARINBody/Data/RotationConstraint` 0.0 0.0 -40.0 40.0 -40.0 40.0 6.0))
      (`BlueprintMapLibrary.Map_Add` _eyerotationconstraint _returnvalue (make `/Game/ARINBody/Data/RotationConstraint` 0.0 0.0 -30.0 30.0 -30.0 30.0 3.0)))
    (:`2.0`
      (`BlueprintMapLibrary.Map_Add` _headrotationconstraint _returnvalue (make `/Game/ARINBody/Data/RotationConstraint` 0.0 0.0 -40.0 40.0 -40.0 40.0 8.0))
      (`BlueprintMapLibrary.Map_Add` _eyerotationconstraint _returnvalue (make `/Game/ARINBody/Data/RotationConstraint` 0.0 0.0 -30.0 30.0 -30.0 30.0 4.0)))))

(fn `LockObjectID`
  (params (ObjectID :type Integer))
  (`self.SetTarget` ObjectID)
  (set `self.Lock` true))

(fn `Relax`
  (params (RelaxTime :type "Float (double-precision)"))
  (set `self.RelaxTime` RelaxTime)
  (set `self.RelaxFlag` true)
  (set `self.GazeFlag` false))

(fn `ReleaseGazeAngle`
  (set `self.IsFixed` false))

(fn `RemapLookAtRotator`
  (params (InRotator :type "Rotator Structure"))
  (returns (OutRotator :type "Rotator Structure"))
  (bind _pitch (.pitch InRotator))
  (bind _yaw (.yaw InRotator))
  (bind _returnvalue (`KismetMathLibrary.SelectFloat` (- _pitch 360.0) _pitch (> _pitch 179.899994)))
  (bind _returnvalue_2 (`KismetMathLibrary.SelectFloat` (- _yaw 360.0) _yaw (> _yaw 179.899994)))
  (return (`KismetMathLibrary.MakeRotator` 0.0 (`KismetMathLibrary.SelectFloat` (+ _returnvalue 360.0) _returnvalue (< _returnvalue -179.899994)) (`KismetMathLibrary.SelectFloat` (+ _returnvalue_2 360.0) _returnvalue_2 (< _returnvalue_2 -179.899994)))))

(fn `Reset`
  (bind _animbpref (`self.AnimBPref`))
  (bind _eyerotationconstraint (`/Game/ARINBody/Blueprints/BP_ARINBody_AnimBlueprint.EyeRotationConstraint` _animbpref))
  (bind _headrotationconstraint (`/Game/ARINBody/Blueprints/BP_ARINBody_AnimBlueprint.HeadRotationConstraint` _animbpref))
  (`BlueprintMapLibrary.Map_Add` _headrotationconstraint "NewEnumerator21" (make `/Game/ARINBody/Data/RotationConstraint` 0.0 0.0 -40.0 40.0 -40.0 40.0 4.0))
  (`BlueprintMapLibrary.Map_Add` _eyerotationconstraint "NewEnumerator21" (make `/Game/ARINBody/Data/RotationConstraint` 0.0 0.0 -30.0 30.0 -30.0 30.0 2.0))
  (`BlueprintMapLibrary.Map_Add` _headrotationconstraint "NewEnumerator13" (make `/Game/ARINBody/Data/RotationConstraint` 0.0 0.0 -40.0 40.0 -40.0 40.0 4.0))
  (`BlueprintMapLibrary.Map_Add` _eyerotationconstraint "NewEnumerator13" (make `/Game/ARINBody/Data/RotationConstraint` 0.0 0.0 -30.0 30.0 -30.0 30.0 2.0))
  (`BlueprintMapLibrary.Map_Add` _headrotationconstraint "NewEnumerator20" (make `/Game/ARINBody/Data/RotationConstraint` 0.0 0.0 -40.0 40.0 -40.0 40.0 4.0))
  (`BlueprintMapLibrary.Map_Add` _eyerotationconstraint "NewEnumerator20" (make `/Game/ARINBody/Data/RotationConstraint` 0.0 0.0 -30.0 30.0 -30.0 30.0 2.0))
  (bind _outactors (`GameplayStatics.GetAllActorsOfClass` "BP_GazeController_C"))
  (for _array_element _outactors
    (`self.UnLockObjectID` _array_element)
    (`self.SetTarget` _array_element 0)
    (`self.Gaze` _array_element)))

(fn `SetPosition`
  (params (ObjectArrayIdx :type Integer) (Position :type "Vector Structure"))
  (bind _characterref (`self.CharacterRef`))
  (if (== ObjectArrayIdx -1)
    (`/Game/ARINBody/Blueprints/CH_ARINBody.SetPositionofIndex` _characterref (`self.ControllerNum`) Position)
    (else
      (`/Game/ARINBody/Blueprints/CH_ARINBody.SetPositionofIndex` _characterref ObjectArrayIdx Position))))

(fn `SetTarget`
  (params (ObjectID :type Integer))
  (if (`self.Lock`)
    _
    (elif (== ObjectID -1)
      (set `self.LookatObjectID` (`self.ControllerNum`))
      (else
        (set `self.LookatObjectID` ObjectID)))))

(fn `UnLockObjectID`
  (set `self.Lock` false))

(fn `UserConstructionScript`)