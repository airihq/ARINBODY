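; BP_JsonDBManager is an actor that loads the motion and sound JSON databases for ARINBody at BeginPlay.
; InitJsonDB parses each array into a map keyed by FileName, using project content data on Android and relative Data paths elsewhere.
; Android still calls LoadFile on external storage but discards those bytes.
; GetData returns string fields from either map, though the Sound branch uses FileName as the field key, ignoring FieldName.
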(event `self.ReceiveBeginPlay`
  (`self.InitJsonDB`))

(fn `GetData`
  (params (DBName :type String) (FileName :type String) (FieldName :type String))
  (returns (Data :type String))
  (switch `string` DBName
    (:`MotionDB`
      (return (`LowEntryJsonLibrary.Object_GetAsStringOrDefault` (`BlueprintMapLibrary.Map_Find` (`self.MotionDB`) FileName) FieldName)))
    (:`SoundDB`
      (return (`LowEntryJsonLibrary.Object_GetAsStringOrDefault` (`BlueprintMapLibrary.Map_Find` (`self.SoundDB`) FileName) FileName)))))

(fn `InitJsonDB`
  (`|ExecutionSequence`
    (:`then_0`
      (if (`LowEntryExtendedStandardLibrary.AndroidPlatform`)
        (bind (_filename _bytes) (`RealTimeImportBPLibrary.LoadFile` "E_ad" "/storage/emulated/0/UE4Game/AICharacter/Data/MotionDB.json"))
        (set `self.MotionDBData` (`LowEntryExtendedStandardLibrary.BytesToStringUtf8` (`LowEntryFileManagerLibrary.GetFileData` (`KismetStringLibrary.Concat_StrStr` (`KismetSystemLibrary.GetProjectContentDirectory`) "ARINBody" "/" "Data" "/" "MotionDB.json"))))
        (else
          (bind (_filename_2 _bytes_2) (`RealTimeImportBPLibrary.LoadFile` "E_gd" "../Data/MotionDB.json"))
          (set `self.MotionDBData` (`LowEntryExtendedStandardLibrary.BytesToStringUtf8` _bytes_2))))
      (bind (_returnjsonobjectvalue _returnjsonarrayvalue) (`LowEntryJsonLibrary.Json_ParseJsonString` (`self.MotionDBData`))
        (:`FoundArray`
          (bind _element (`/LowEntryJson/Blueprints/LowEntryJsonMacros.JsonArrayForEachLoop` _returnjsonarrayvalue)
            (:`LoopBody`
              (bind _returnvalue (`LowEntryJsonLibrary.Value_GetAsJsonObjectOrDefault` _element))
              (`BlueprintMapLibrary.Map_Add` (`self.MotionDB`) (`LowEntryJsonLibrary.Object_GetAsStringOrDefault` _returnvalue "FileName") _returnvalue))))))
    (:`then_1`
      (if (`LowEntryExtendedStandardLibrary.AndroidPlatform`)
        (bind (_filename_3 _bytes_3) (`RealTimeImportBPLibrary.LoadFile` "E_ad" "/storage/emulated/0/UE4Game/AICharacter/Data/Sound.json"))
        (set `self.SoundDBData` (`LowEntryExtendedStandardLibrary.BytesToStringUtf8` (`LowEntryFileManagerLibrary.GetFileData` (`KismetStringLibrary.Concat_StrStr` (`KismetSystemLibrary.GetProjectContentDirectory`) "ARINBody" "/" "Data" "/" "Sound.json"))))
        (else
          (bind (_filename_4 _bytes_4) (`RealTimeImportBPLibrary.LoadFile` "E_gd" "../Data/Sound.json"))
          (set `self.SoundDBData` (`LowEntryExtendedStandardLibrary.BytesToStringUtf8` _bytes_4))))
      (bind (_returnjsonobjectvalue_2 _returnjsonarrayvalue_2) (`LowEntryJsonLibrary.Json_ParseJsonString` (`self.SoundDBData`))
        (:`FoundArray`
          (bind _element_2 (`/LowEntryJson/Blueprints/LowEntryJsonMacros.JsonArrayForEachLoop` _returnjsonarrayvalue_2)
            (:`LoopBody`
              (bind _returnvalue_2 (`LowEntryJsonLibrary.Value_GetAsJsonObjectOrDefault` _element_2))
              (`BlueprintMapLibrary.Map_Add` (`self.SoundDB`) (`LowEntryJsonLibrary.Object_GetAsStringOrDefault` _returnvalue_2 "FileName") _returnvalue_2))))))))

(fn `UserConstructionScript`)