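; BP_GazeUpperController turns the ARIN body character's upper gaze toward indexed target positions stored on CH_ARINBody.
; DoStroke computes clamped yaw and pitch to the target, deriving a duration if none is given, and DoRelax returns to zero.
; Tick interpolates both angles into the AnimBP, drives this controller's blend alpha and sets completion flags.
; An interrupt event bound on the AnimBP forces a quick relax, overriding the current state.
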(event `self.ReceiveBeginPlay`
  ;[1 1 1] BeginPlayEvent(Initialize ARINBodyAnimBP Reference)
  (`|ExecutionSequence`
    (:`then_0`
      (bind _outactors (`GameplayStatics.GetAllActorsOfClass` "/Game/ARINBody/Blueprints/CH_ARINBody.CH_ARINBody_C"))
      (for _array_element _outactors
        (bind _asbp_arinbody_anim_blueprint (cast `/Game/ARINBody/Blueprints/BP_ARINBody_AnimBlueprint` (`SkeletalMeshComponent.GetAnimInstance` (`Character.Mesh` _array_element))))
        (bind _output_get (set `self.AnimBPref` _asbp_arinbody_anim_blueprint))
        (add `/Game/ARINBody/Blueprints/BP_ARINBody_AnimBlueprint.InterruptAnimation` _output_get (delegate `InterruptEvent`))))
    (:`then_1`
      (bind _outactors_2 (`GameplayStatics.GetAllActorsOfClass` "/Game/ARINBody/Blueprints/CH_ARINBody.CH_ARINBody_C"))
      (for _array_element_2 _outactors_2
        (set `self.CharacterRef` _array_element_2)))
    (:`then_2`
      (set `self.ControllerNum` (`KismetMathLibrary.Conv_ByteToInt` (enumliteral `/Game/ARINBody/Data/ControllerNameEnum` "NewEnumerator21"))))
    (:`then_4`
      (set `self.ObjectID` (`self.ControllerNum`)))))

(event `InterruptEvent`
  ;[1 1 1] BeginPlayEvent(Initialize ARINBodyAnimBP Reference)
  (`self.DoInterruptRelax`))

(event `self.ReceiveTick`
  (params (DeltaSeconds :type "Float (single-precision)"))
  (bind _controllerblendalphaarray (`/Game/ARINBody/Blueprints/BP_ARINBody_AnimBlueprint.ControllerBlendAlphaArray` (`self.AnimBPref`)))
  ;[1 1 1] TickEvent(Interpolation Angle Parameters)
  (if (`self.InterruptFlag`)
    (`KismetArrayLibrary.Array_Set` (`/Game/ARINBody/Blueprints/BP_ARINBody_AnimBlueprint.ControllerBlendAlphaArray` (`self.AnimBPref`)) (`self.ControllerNum`) (+ (`|GetArrayItem` (`/Game/ARINBody/Blueprints/BP_ARINBody_AnimBlueprint.ControllerBlendAlphaArray` (`self.AnimBPref`)) (`self.ControllerNum`)) (/ (`GameplayStatics.GetWorldDeltaSeconds`) (`self.StrokeTime`))))
    (set `/Game/ARINBody/Blueprints/BP_ARINBody_AnimBlueprint.GazeUpperAngleX` (`KismetMathLibrary.FInterpTo_Constant` (`/Game/ARINBody/Blueprints/BP_ARINBody_AnimBlueprint.GazeUpperAngleX` (`self.AnimBPref`)) (`self.TargetAngleX`) (`GameplayStatics.GetWorldDeltaSeconds`) (/ (`KismetMathLibrary.Abs` (- (`self.TargetAngleX`) (`self.CurAngleX`))) (`self.StrokeTime`))) (`self.AnimBPref`))
    (set `/Game/ARINBody/Blueprints/BP_ARINBody_AnimBlueprint.GazeUpperAngleY` (`KismetMathLibrary.FInterpTo_Constant` (`/Game/ARINBody/Blueprints/BP_ARINBody_AnimBlueprint.GazeUpperAngleY` (`self.AnimBPref`)) (`self.TargetAngleY`) (`GameplayStatics.GetWorldDeltaSeconds`) (/ (`KismetMathLibrary.Abs` (- (`self.TargetAngleY`) (`self.CurAngleY`))) (`self.StrokeTime`))) (`self.AnimBPref`))
    (if (>= (`|GetArrayItem` (`/Game/ARINBody/Blueprints/BP_ARINBody_AnimBlueprint.ControllerBlendAlphaArray` (`self.AnimBPref`)) (`self.ControllerNum`)) 1.0)
      (set `self.CurAngleX` (`self.TargetAngleX`))
      (set `self.CurAngleY` (`self.TargetAngleY`))
      (set `self.State` 0)
      (set `self.TurnFlag` 1)
      (set `self.GazeFlag` 1)
      (set `self.GazeUpperFlag` 1)
      (`KismetArrayLibrary.Array_Set` (`/Game/ARINBody/Blueprints/BP_ARINBody_AnimBlueprint.ControllerBlendAlphaArray` (`self.AnimBPref`)) (`self.ControllerNum`) 1.0)
      (set `self.InterruptFlag` false))
    (else
      (switch `int` (`self.State`)
        (:`1`
          (if (> (`|GetArrayItem` (`/Game/ARINBody/Blueprints/BP_ARINBody_AnimBlueprint.ControllerBlendAlphaArray` (`self.AnimBPref`)) (`self.ControllerNum`)) 0.0)
            (`KismetArrayLibrary.Array_Set` _controllerblendalphaarray (`self.ControllerNum`) (- (`|GetArrayItem` _controllerblendalphaarray (`self.ControllerNum`)) (/ (`GameplayStatics.GetWorldDeltaSeconds`) (`self.StrokeTime`)))))
          (set `/Game/ARINBody/Blueprints/BP_ARINBody_AnimBlueprint.GazeUpperAngleX` (`KismetMathLibrary.FInterpTo_Constant` (`/Game/ARINBody/Blueprints/BP_ARINBody_AnimBlueprint.GazeUpperAngleX` (`self.AnimBPref`)) (`self.TargetAngleX`) (`GameplayStatics.GetWorldDeltaSeconds`) (/ (`KismetMathLibrary.Abs` (- (`self.TargetAngleX`) (`self.CurAngleX`))) (`self.StrokeTime`))) (`self.AnimBPref`))
          (set `/Game/ARINBody/Blueprints/BP_ARINBody_AnimBlueprint.GazeUpperAngleY` (`KismetMathLibrary.FInterpTo_Constant` (`/Game/ARINBody/Blueprints/BP_ARINBody_AnimBlueprint.GazeUpperAngleY` (`self.AnimBPref`)) (`self.TargetAngleY`) (`GameplayStatics.GetWorldDeltaSeconds`) (/ (`KismetMathLibrary.Abs` (- (`self.TargetAngleY`) (`self.CurAngleY`))) (`self.StrokeTime`))) (`self.AnimBPref`))
          (if (and (`KismetMathLibrary.NearlyEqual_FloatFloat` (`/Game/ARINBody/Blueprints/BP_ARINBody_AnimBlueprint.GazeUpperAngleX` (`self.AnimBPref`)) (`self.TargetAngleX`) 0.1) (`KismetMathLibrary.NearlyEqual_FloatFloat` (`/Game/ARINBody/Blueprints/BP_ARINBody_AnimBlueprint.GazeUpperAngleY` (`self.AnimBPref`)) (`self.TargetAngleY`) 0.1))
            (set `self.CurAngleX` (`self.TargetAngleX`))
            (set `self.CurAngleY` (`self.TargetAngleY`))
            (set `self.State` 0)
            (set `self.TurnFlag` 1)
            (set `self.GazeFlag` 1)
            (set `self.GazeUpperFlag` 1)))
        (:`2`
          (`KismetArrayLibrary.Array_Set` (`/Game/ARINBody/Blueprints/BP_ARINBody_AnimBlueprint.ControllerBlendAlphaArray` (`self.AnimBPref`)) (`self.ControllerNum`) (+ (`|GetArrayItem` (`/Game/ARINBody/Blueprints/BP_ARINBody_AnimBlueprint.ControllerBlendAlphaArray` (`self.AnimBPref`)) (`self.ControllerNum`)) (/ (`GameplayStatics.GetWorldDeltaSeconds`) (`self.StrokeTime`))))
          (set `/Game/ARINBody/Blueprints/BP_ARINBody_AnimBlueprint.GazeUpperAngleX` (`KismetMathLibrary.FInterpTo_Constant` (`/Game/ARINBody/Blueprints/BP_ARINBody_AnimBlueprint.GazeUpperAngleX` (`self.AnimBPref`)) (`self.TargetAngleX`) (`GameplayStatics.GetWorldDeltaSeconds`) (/ (`KismetMathLibrary.Abs` (- (`self.TargetAngleX`) (`self.CurAngleX`))) (`self.StrokeTime`))) (`self.AnimBPref`))
          (set `/Game/ARINBody/Blueprints/BP_ARINBody_AnimBlueprint.GazeUpperAngleY` (`KismetMathLibrary.FInterpTo_Constant` (`/Game/ARINBody/Blueprints/BP_ARINBody_AnimBlueprint.GazeUpperAngleY` (`self.AnimBPref`)) (`self.TargetAngleY`) (`GameplayStatics.GetWorldDeltaSeconds`) (/ (`KismetMathLibrary.Abs` (- (`self.TargetAngleY`) (`self.CurAngleY`))) (`self.StrokeTime`))) (`self.AnimBPref`))
          (if (and (`KismetMathLibrary.NearlyEqual_FloatFloat` (`/Game/ARINBody/Blueprints/BP_ARINBody_AnimBlueprint.GazeUpperAngleX` (`self.AnimBPref`)) (`self.TargetAngleX`) 0.1) (`KismetMathLibrary.NearlyEqual_FloatFloat` (`/Game/ARINBody/Blueprints/BP_ARINBody_AnimBlueprint.GazeUpperAngleY` (`self.AnimBPref`)) (`self.TargetAngleY`) 0.1) (>= (`|GetArrayItem` (`/Game/ARINBody/Blueprints/BP_ARINBody_AnimBlueprint.ControllerBlendAlphaArray` (`self.AnimBPref`)) (`self.ControllerNum`)) 1.0))
            (set `self.CurAngleX` (`self.TargetAngleX`))
            (set `self.CurAngleY` (`self.TargetAngleY`))
            (set `self.State` 0)
            (set `self.TurnFlag` 1)
            (set `self.GazeFlag` 1)
            (set `self.GazeUpperFlag` 1)
            (`KismetArrayLibrary.Array_Set` (`/Game/ARINBody/Blueprints/BP_ARINBody_AnimBlueprint.ControllerBlendAlphaArray` (`self.AnimBPref`)) (`self.ControllerNum`) 1.0)))))))

(fn `DoInterruptRelax`
  (set `self.InterruptFlag` true)
  (set `self.TargetAngleX` 0.0)
  (set `self.TargetAngleY` 0.0)
  (set `self.StrokeTime` 0.5)
  (set `self.RelaxTimer` 0.0))

(fn `DoRelax`
  (params (RelaxTime :type "Float (double-precision)"))
  (if (<= (`|GetArrayItem` (`/Game/ARINBody/Blueprints/BP_ARINBody_AnimBlueprint.ControllerBlendAlphaArray` (`self.AnimBPref`)) (`self.ControllerNum`)) 0.0)
    (if (== (`self.State`) 0)
      ;[1 1 1] Set Angles and Timer 0 and Relax Start
      (set `self.State` 2)
      (set `self.TargetAngleX` 0.0)
      (set `self.TargetAngleY` 0.0)
      (set `self.StrokeTime` RelaxTime)
      (set `self.RelaxTimer` 0.0)
      (set `self.PrepTimer` 0.0)
      ;[1 1 1] If Input Time is Negative Set  Anim Time 1.0
      (if (< (`self.StrokeTime`) 0.0)
        (set `self.StrokeTime` 1.0)))))

(fn `DoStroke`
  (params (ObjectID :type Integer) (GazeAnimTime :type "Float (double-precision)"))
  (bind (_returnvalue_roll _returnvalue_pitch _returnvalue_yaw) (`KismetMathLibrary.BreakRotator` (`SceneComponent.K2_GetComponentRotation` (`Actor.RootComponent` (`self.CharacterRef`)))))
  (bind _returnvalue (- 180.0 (- (`KismetMathLibrary.Abs` (`self.TargetAngleX`)) 180.0)))
  (bind (_returnvalue_roll_2 _returnvalue_pitch_2 _returnvalue_yaw_2) (`KismetMathLibrary.BreakRotator` (`KismetMathLibrary.FindLookAtRotation` (+ (`SceneComponent.K2_GetComponentLocation` (`Actor.RootComponent` (`self.CharacterRef`))) (0.0 0.0 80.0)) (`BlueprintMapLibrary.Map_Find` (`/Game/ARINBody/Blueprints/CH_ARINBody.ObjectArray` (`self.CharacterRef`)) (`self.ObjectID`)))))
  (if (== (`self.State`) 0)
    ;[1 1 1] Set Target ID and Animation Time
    (if (== ObjectID -1)
      (set `self.ObjectID` (`self.ControllerNum`))
      (else
        (set `self.ObjectID` ObjectID)))
    (if (not (`.ReturnValue` (`BlueprintMapLibrary.Map_Find` (`/Game/ARINBody/Blueprints/CH_ARINBody.ObjectArray` (`self.CharacterRef`)) (`self.ObjectID`))))
      (set `self.ObjectID` (`self.ControllerNum`)))
    (set `self.StrokeTime` GazeAnimTime)
    ;[1 1 1] Calculate and Set X axis Angle
    (bind _output_get (set `self.TargetAngleX` (- _returnvalue_yaw_2 _returnvalue_yaw)))
    (if (> (`KismetMathLibrary.Abs` (`self.TargetAngleX`)) 180.0)
      (if (> (`self.TargetAngleX`) 0.0)
        (set `self.TargetAngleX` (`KismetMathLibrary.FClamp` (* _returnvalue -1.0) -80.0 80.0))
        (else
          (set `self.TargetAngleX` (`KismetMathLibrary.FClamp` _returnvalue -80.0 80.0))))
      (else
        (set `self.TargetAngleX` (`KismetMathLibrary.FClamp` _output_get -80.0 80.0))))
    ;[1 1 1] Set Y Angle
    (set `self.TargetAngleY` (`KismetMathLibrary.FClamp` _returnvalue_pitch_2 -65.0 65.0))
    ;[1 1 1] Calculate Animation Time When Input time is negative
    (if (<= (`self.StrokeTime`) 0.0)
      (set `self.StrokeTime` (`KismetMathLibrary.FClamp` (/ (`KismetMathLibrary.FMax` (- (`self.TargetAngleX`) (`self.CurAngleX`)) (- (`self.TargetAngleY`) (`self.CurAngleY`))) 40.0) 0.5 2.0)))
    ;[1 1 1] Start Gaze and Set Flags
    (set `self.State` 1)
    (`KismetArrayLibrary.Array_Set` (`/Game/ARINBody/Blueprints/BP_ARINBody_AnimBlueprint.ControllerBlendAlphaArray` (`self.AnimBPref`)) (`self.ControllerNum`))
    (set `self.TurnFlag` 0)
    (set `self.GazeFlag` 0)
    (set `self.GazeUpperFlag` 0)))

(fn `Setposition`
  (params (ObjectArrayIdx :type Integer) (Position :type "Vector Structure"))
  (bind _characterref (`self.CharacterRef`))
  (if (== ObjectArrayIdx -1)
    (`/Game/ARINBody/Blueprints/CH_ARINBody.SetPositionofIndex` _characterref (`self.ControllerNum`) Position)
    (else
      (`/Game/ARINBody/Blueprints/CH_ARINBody.SetPositionofIndex` _characterref ObjectArrayIdx Position))))

(fn `UserConstructionScript`)