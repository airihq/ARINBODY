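; Face controller for the ARIN body that animates named expressions as morph targets on player character 0's mesh.
; Expressions load as blend-shape maps from the FaceExpressionList data table, and CallStroke, CallHold, CallRelax or CallRelaxByInterrupt selects a timed phase.
; Tick runs PlayFacialExpression, blending linearly from previous to target on stroke and back to Neutral on relax, using snapshotted live weights when interrupted.
; Older frame-based and stroke-relax players remain but are not run.
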(event `self.ReceiveTick`
  (params (DeltaSeconds :type "Float (single-precision)"))
  (`self.PlayFacialExpression`))

(fn `CallHold`
  (params (FaceExpression :type String) (duration :type "Float (double-precision)"))
  (`self.SelectFaceExpMap` FaceExpression)
  (`|ExecutionSequence`
    (:`then_0`
      (set `self.IsPeriodic` false))
    (:`then_1`
      (set `self.TimeHold` 0.0)
      (set `self.TimeHoldMax` duration))
    (:`then_2`
      (set `self.bPlayAnimation` true))
    (:`then_3`
      (set `self.bPlayStroke` false)
      (set `self.bPlayHold` true)
      (set `self.bPlayRelax` false))
    (:`then_4`
      (set `self.bPlayRelaxByInterrupt` false))))

(fn `CallRelax`
  (params (FaceExpression :type String) (duration :type "Float (double-precision)"))
  (`self.SelectFaceExpMap` FaceExpression)
  (`|ExecutionSequence`
    (:`then_0`
      (set `self.IsPeriodic` false))
    (:`then_1`
      (set `self.TimeRelax` 0.0)
      (set `self.TimeRelaxMax` duration))
    (:`then_2`
      (set `self.bPlayAnimation` true))
    (:`then_3`
      (set `self.bPlayStroke` false)
      (set `self.bPlayHold` false)
      (set `self.bPlayRelax` true))
    (:`then_4`
      (set `self.bPlayRelaxByInterrupt` false))))

(fn `CallRelaxByInterrupt`
  (params (FaceExpression :type String) (Duration :type "Float (double-precision)"))
  (`self.SelectFaceExpMap` FaceExpression)
  ;[1 1 1] Save current weight values
  (`self.GetCurrentWeightsFaceMorphMaps`)
  (`|ExecutionSequence`
    (:`then_0`
      (set `self.IsPeriodic` false))
    (:`then_1`
      (set `self.TimeRelax` 0.0)
      (set `self.TimeRelaxMax` Duration))
    (:`then_2`
      (set `self.bPlayAnimation` true))
    (:`then_3`
      (set `self.bPlayStroke` false)
      (set `self.bPlayHold` false)
      (set `self.bPlayRelax` false))
    (:`then_4`
      (set `self.bPlayRelaxByInterrupt` true))))

(fn `CallStroke`
  (params (FaceExpression :type String) (duration :type "Float (double-precision)"))
  (`self.SelectFaceExpMap` FaceExpression)
  (`|ExecutionSequence`
    (:`then_1`
      (set `self.TimeStroke` 0.0)
      (set `self.TimeStrokeMax` duration))
    (:`then_2`
      (set `self.bPlayAnimation` true))
    (:`then_3`
      (set `self.bPlayStroke` true)
      (set `self.bPlayHold` false)
      (set `self.bPlayRelax` false))
    (:`then_4`
      (set `self.bPlayRelaxByInterrupt` false))))

(fn `GetCurrentWeightsFaceMorphMaps`
  (`BlueprintMapLibrary.Map_Clear` (`self.CurrentWeightMap`))
  (bind _keys (`BlueprintMapLibrary.Map_Keys` (`self.FaceMorphMap`)))
  (for _array_element _keys
    (`BlueprintMapLibrary.Map_Add` (`self.CurrentWeightMap`) _array_element (`SkeletalMeshComponent.GetMorphTarget` (`Character.Mesh` (`GameplayStatics.GetPlayerCharacter` 0)) (`KismetStringLibrary.Conv_StringToName` _array_element)))))

(fn `InitARINBodyFaceController`
  (params (ARINBodyCharacter :type "/Game/ARINBody/Blueprints/CH_ARINBody Object Reference"))
  (set `self.ARINBodyCharacterRef` ARINBodyCharacter))

(fn `InitMorphMap`
  (bind _returnvalue (`|GetDataTableRow` "/Game/ARINBody/Data/faceExpressionList.faceExpressionList" "Neutral")
    (:`then`
      (bind _output_get (set `self.FaceMorphMap` (`.BlendShape_4_95E969E7486BA2FDCAEE4997F0AEB81F` (break `/Game/ARINBody/Data/FaceExpStruct` _returnvalue))))
      (bind _output_get_2 (set `self.PrevFaceMorphMap` _output_get))
      (set `self.NeutralFaceMorphMap` _output_get_2))))

(fn `PlayAnimation`
  (params (FaceExpression :type String) (IsPeriodic :type Boolean) (TimeStroke :type "Float (double-precision)") (TimeHold :type "Float (double-precision)") (TimeRelax :type "Float (double-precision)"))
  (`self.SelectFaceExpMap` FaceExpression)
  (`|ExecutionSequence`
    (:`then_0`
      (set `self.IsPeriodic` IsPeriodic))
    (:`then_1`
      (set `self.TimeStrokeMax` TimeStroke)
      (set `self.TimeHoldMax` TimeHold)
      (set `self.TimeRelaxMax` TimeRelax))
    (:`then_2`
      (set `self.TimeStroke` 0.0)
      (set `self.TimeHold` 0.0)
      (set `self.TimeRelax` 0.0))
    (:`then_3`
      (set `self.bPlayAnimation` true))))

(fn `PlayFaceExpression`
  (if (`self.bPlayAnimation`)
    (bind _output_get (set `self.TimeStroke` (+ (`self.TimeStroke`) (`GameplayStatics.GetWorldDeltaSeconds`))))
    (if (<= _output_get (`self.TimeStrokeMax`))
      (`self.SetFaceMorphMap` (/ (`self.TimeStroke`) (`self.TimeStrokeMax`)))
      (else
        (bind _output_get_2 (set `self.TimeRelax` (+ (`self.TimeRelax`) (`GameplayStatics.GetWorldDeltaSeconds`))))
        (if (<= _output_get_2 (`self.TimeRelaxMax`))
          (`self.SetFaceMorphMap` (- 1.0 (/ (`self.TimeRelax`) (`self.TimeRelaxMax`))))
          (else
            (set `self.bPlayAnimation` false)))))))

(fn `PlayFaceMorphAnimation`
  (bind _framenummax (`self.FrameNumMax`))
  (bind _facemorphmap (`self.FaceMorphMap`))
  (bind _returnvalue (`KismetMathLibrary.Conv_IntToDouble` _framenummax))
  (bind _mesh (`Character.Mesh` (`GameplayStatics.GetPlayerCharacter` 0)))
  (if (`self.bPlayAnimation`)
    (bind _result (`/Engine/EditorBlueprintResources/StandardMacros.IncrementInt` (`self.FrameNum`))
      (:`  `
        (if (<= _result (`KismetMathLibrary.FTrunc` (`KismetMathLibrary.Conv_IntToDouble` _framenummax)))
          (bind _keys (`BlueprintMapLibrary.Map_Keys` _facemorphmap))
          (for _array_element _keys
            (bind _returnvalue_2 (`KismetMathLibrary.Conv_IntToDouble` _result))
            (`SkeletalMeshComponent.SetMorphTarget` _mesh (`KismetStringLibrary.Conv_StringToName` _array_element) (* (/ (`BlueprintMapLibrary.Map_Find` _facemorphmap _array_element) (`KismetMathLibrary.Conv_IntToDouble` _framenummax)) _returnvalue_2) true))
          (else
            (bind _returnvalue_3 (- (* _returnvalue 2.0) _returnvalue_2))
            (if (>= _returnvalue_3 0.0)
              (bind _keys_2 (`BlueprintMapLibrary.Map_Keys` _facemorphmap))
              (for _array_element_2 _keys_2
                (`SkeletalMeshComponent.SetMorphTarget` _mesh (`KismetStringLibrary.Conv_StringToName` _array_element_2) (* (`BlueprintMapLibrary.Map_Find` _facemorphmap _array_element_2) (/ _returnvalue_3 _returnvalue)) true)))))))))

(fn `PlayFacialExpression`
  (if (`self.bPlayAnimation`)
    (`|ExecutionSequence`
      (:`then_0`
        (if (`self.bPlayStroke`)
          ;[1 1 1] Stroke Animation
          (bind _output_get (set `self.TimeStroke` (+ (`self.TimeStroke`) (`GameplayStatics.GetWorldDeltaSeconds`))))
          (if (<= _output_get (`self.TimeStrokeMax`))
            (`self.TransformFaceMorphMaps` (/ (`self.TimeStroke`) (`self.TimeStrokeMax`)) (`self.PrevFaceMorphMap`) (`self.FaceMorphMap`))
            (else
              (set `self.PrevFaceMorphMap` (`self.FaceMorphMap`))
              (set `self.bPlayStroke` false)
              (set `self.bPlayAnimation` false)))))
      (:`then_1`
        (if (`self.bPlayHold`)
          ;[1 1 1] hold animation
          (bind _output_get_2 (set `self.TimeHold` (+ (`self.TimeHold`) (`GameplayStatics.GetWorldDeltaSeconds`))))
          (if (not (>= _output_get_2 (`self.TimeHoldMax`)))
            (set `self.bPlayHold` false)
            (set `self.bPlayAnimation` false))))
      (:`then_2`
        (if (`self.bPlayRelax`)
          ;[1 1 1] relax animation
          (bind _output_get_3 (set `self.TimeRelax` (+ (`self.TimeRelax`) (`GameplayStatics.GetWorldDeltaSeconds`))))
          (if (<= _output_get_3 (`self.TimeRelaxMax`))
            (`self.TransformFaceMorphMaps` (- 1.0 (/ (`self.TimeRelax`) (`self.TimeRelaxMax`))) (`self.NeutralFaceMorphMap`) (`self.FaceMorphMap`))
            (else
              (set `self.bPlayRelax` false)
              (set `self.bPlayAnimation` false)
              (set `self.PrevFaceMorphMap` (`self.NeutralFaceMorphMap`))))))
      (:`then_3`
        (if (`self.bPlayRelaxByInterrupt`)
          ;[1 1 1] relax animation by interrupt
          (bind _output_get_4 (set `self.TimeRelax` (+ (`self.TimeRelax`) (`GameplayStatics.GetWorldDeltaSeconds`))))
          (if (<= _output_get_4 (`self.TimeRelaxMax`))
            (`self.TransformFaceMorphMaps` (- 1.0 (/ (`self.TimeRelax`) (`self.TimeRelaxMax`))) (`self.NeutralFaceMorphMap`) (`self.CurrentWeightMap`))
            (else
              (set `self.bPlayRelaxByInterrupt` false)
              (set `self.bPlayAnimation` false)
              (set `self.PrevFaceMorphMap` (`self.NeutralFaceMorphMap`)))))))))

(fn `PlayRandomAnimation`
  (`self.SetRandomFaceExpMap`)
  (set `self.bPlayAnimation` true)
  (set `self.FrameNum` 1)
  (set `self.FrameNumMax` 50))

(fn `SelectFaceExpMap`
  (params (SelectedExpressionName :type String))
  (bind _returnvalue (`|GetDataTableRow` "/Game/ARINBody/Data/faceExpressionList.faceExpressionList" (`KismetStringLibrary.Conv_StringToName` SelectedExpressionName))
    (:`then`
      (set `self.FaceMorphMap` (`.BlendShape_4_95E969E7486BA2FDCAEE4997F0AEB81F` (break `/Game/ARINBody/Data/FaceExpStruct` _returnvalue))))))

(fn `SetFaceMorphMap`
  (params (weight :type "Float (double-precision)"))
  (bind _facemorphmap (`self.FaceMorphMap`))
  (bind _keys (`BlueprintMapLibrary.Map_Keys` _facemorphmap))
  (for _array_element _keys
    (`SkeletalMeshComponent.SetMorphTarget` (`Character.Mesh` (`GameplayStatics.GetPlayerCharacter` 0)) (`KismetStringLibrary.Conv_StringToName` _array_element) (* (`BlueprintMapLibrary.Map_Find` _facemorphmap _array_element) weight) true)))

(fn `SetRandomFaceExpMap`
  (bind _outrownames (`DataTableFunctionLibrary.GetDataTableRowNames` "/Game/ARINBody/Data/faceExpressionList.faceExpressionList"))
  (bind _returnvalue (`|GetDataTableRow` "/Game/ARINBody/Data/faceExpressionList.faceExpressionList" (`|GetArrayItem` _outrownames (`KismetMathLibrary.RandomInteger` (`KismetArrayLibrary.Array_Length` _outrownames))))
    (:`then`
      (set `self.FaceMorphMap` (`.BlendShape_4_95E969E7486BA2FDCAEE4997F0AEB81F` (break `/Game/ARINBody/Data/FaceExpStruct` _returnvalue))))))

(fn `TransformFaceMorphMaps`
  (params (weight :type "Float (double-precision)") (SourceFaceMap :type "Map of String to Float (double-precision)") (TargetFaceMap :type "Map of String to Float (double-precision)"))
  (bind _keys (`BlueprintMapLibrary.Map_Keys` SourceFaceMap))
  (for _array_element _keys
    (`SkeletalMeshComponent.SetMorphTarget` (`Character.Mesh` (`GameplayStatics.GetPlayerCharacter` 0)) (`KismetStringLibrary.Conv_StringToName` _array_element) (+ (* (`BlueprintMapLibrary.Map_Find` TargetFaceMap _array_element) weight) (* (`BlueprintMapLibrary.Map_Find` SourceFaceMap _array_element) (- 1.0 weight))) true)))

(fn `TransformFaceMorphMapsToNeutral`
  (params (weight :type "Float (double-precision)"))
  (bind _neutralfacemorphmap (`self.NeutralFaceMorphMap`))
  (bind _keys (`BlueprintMapLibrary.Map_Keys` _neutralfacemorphmap))
  (for _array_element _keys
    (`SkeletalMeshComponent.SetMorphTarget` (`Character.Mesh` (`GameplayStatics.GetPlayerCharacter` 0)) (`KismetStringLibrary.Conv_StringToName` _array_element) (+ (* (`BlueprintMapLibrary.Map_Find` _neutralfacemorphmap _array_element) weight) 1.0) true)))

(fn `UserConstructionScript`)